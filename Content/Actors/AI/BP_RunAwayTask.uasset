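; Behavior tree task that picks a flee destination for an AI pawn away from the bomb in the NearbyBomb blackboard key.
; It scales the bomb-to-pawn vector by 1000, uses it directly as the world-space origin of a random reachable point search, and writes the result to TargetLocation.
; It prints a debug string and finishes successfully, but never finishes if the bomb cast fails.
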(event `self.ReceiveExecuteAI`
  (params (OwnerController :type "AIController Object Reference") (ControlledPawn :type "Pawn Object Reference"))
  (bind _asactor (cast `Actor` (`BTFunctionLibrary.GetBlackboardValueAsObject` (`self.NearbyBomb`))))
  (`BTFunctionLibrary.SetBlackboardValueAsVector` (`self.TargetLocation`) (`NavigationSystemV1.K2_GetRandomReachablePointInRadius` (* (- (`Actor.K2_GetActorLocation` ControlledPawn) (`Actor.K2_GetActorLocation` _asactor)) 1000.0) (`self.Radius`) null null))
  (`KismetSystemLibrary.PrintString` "RUNNN")
  (`self.FinishExecute` true))